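; BP_FuseLock is a two-slot fuse lock that shows which fuses are in place and signals when both are set.
; The RequiredFuses boolean array drives the visibility of Fuse0 and Fuse1, and an explosion emitter spawns at FuseCenter when both entries are true.
; FuseUpdate plays a pickup sound, then reuses the BeginPlay refresh chain.
; The Blueprint only reads RequiredFuses and contains no door or unlock logic.
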(event EventBeginPlay
  (bind _requiredfuses (Variables|Default|GetRequiredFuses))
  (bind _output (Utilities|Array|Get(acopy) _requiredfuses))
  (bind _output_2 (Utilities|Array|Get(acopy) _requiredfuses 1))
  ;[1 0 0.5482] Set the visibility of different fuse elements
  (Rendering|SetVisibility (Variables|Default|GetFuse_0) _output false)
  (Rendering|SetVisibility (Variables|Default|GetFuse_1) _output_2 false)
  ;[1 0 0.5482] If fuse unlocked, launch particle
  (if (and _output _output_2)
    (Effects|SpawnEmitteratLocation "/Game/StarterContent/Particles/P_Explosion.P_Explosion" (Transformation|GetWorldLocation (Variables|Default|GetFuse%20Center)) "0, 0, 0" "2.000000,2.000000,2.000000")))

(event EventFuseUpdate
  (bind _requiredfuses (Variables|Default|GetRequiredFuses))
  (bind _output (Utilities|Array|Get(acopy) _requiredfuses))
  (bind _output_2 (Utilities|Array|Get(acopy) _requiredfuses 1))
  ;[0 1 0.1445] Play Fuse Sound
  (Audio|PlaySoundatLocation "/Game/Sounds/item_pickup.item_pickup" (Transformation|GetWorldLocation (Variables|Default|GetFuse%20Center)) "0, 0, 0" 0.3)
  ;[1 0 0.5482] Set the visibility of different fuse elements
  (Rendering|SetVisibility (Variables|Default|GetFuse_0) _output false)
  (Rendering|SetVisibility (Variables|Default|GetFuse_1) _output_2 false)
  ;[1 0 0.5482] If fuse unlocked, launch particle
  (if (and _output _output_2)
    (Effects|SpawnEmitteratLocation "/Game/StarterContent/Particles/P_Explosion.P_Explosion" (Transformation|GetWorldLocation (Variables|Default|GetFuse%20Center)) "0, 0, 0" "2.000000,2.000000,2.000000")))

(fn ConstructionScript)