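; BP_Torch is a torch actor whose light can be switched on and off.
; ChangeTorchState toggles the Light component's visibility and plays a click sound at the shared root's location.
; It then reads the light's visibility to set the OnOrOff scalar parameter on the cap mesh's materials, keeping their look in step with the light.
; The event graph and construction script contain no logic.
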(event EventBeginPlay)

(event Collision|EventActorBeginOverlap
  (params (OtherActor :type Actor%20Object%20Reference)))

(event EventTick
  (params (DeltaSeconds :type Float%20%28single-precision%29)))

(fn ConstructionScript)

(fn ChangeTorchState
  (bind _sm_cap (Variables|Default|GetSM_Cap))
  ;[1 0 0.5482] Turn Light On/Off
  (Rendering|ToggleVisibility (Variables|Default|GetLight) false)
  ;[0 1 0.1445] Play Audio
  (Audio|PlaySoundatLocation "/Game/Sounds/light_click.light_click" (Transformation|GetWorldLocation (Variables|Default|GetSharedRoot)) "0, 0, 0" 0.3 0.8)
  ;[1 0.1522 0] Change Material Depending On State
  (if (Rendering|IsVisible (Variables|Default|GetLight))
    (Rendering|Material|SetScalarParameterValueonMaterials _sm_cap "OnOrOff" 1.0)
    (else
      (Rendering|Material|SetScalarParameterValueonMaterials _sm_cap "OnOrOff" 0.0))))