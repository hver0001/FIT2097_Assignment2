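; BP_Door is a toggleable door that swings open and shut and shows its lock state through its material.
; When toggled while CanBeOpened is true, it plays or reverses a rotation timeline on the mesh and plays a creak sound.
; Tick derives ClosedDoor from the timeline angle to choose the direction.
; BeginPlay and WasUnlocked apply the locked or unlocked material from IsLocked.
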(event EventTick
  (params (DeltaSeconds :type Float%20%28single-precision%29))
  ;[1 0 0.5482] Animate Door Opening
  (Variables|Default|SetClosedDoor (< (stale EventWasToggled _rotation_angle) 1.0)))

(event EventWasUnlocked
  (bind _sm_door (Variables|Default|GetSM_Door))
  ;[1 0.1522 0] Change Material Depending on State
  (if (Class|Door|IsLocked)
    (Rendering|Material|SetMaterial _sm_door 0 (Variables|Default|GetLockedMaterial))
    (else
      (Rendering|Material|SetMaterial _sm_door 0 (Variables|Default|GetUnlockedMaterial)))))

(event EventBeginPlay
  (bind _sm_door (Variables|Default|GetSM_Door))
  ;[1 0.1522 0] Change Material Depending on State
  (if (Class|Door|IsLocked)
    (Rendering|Material|SetMaterial _sm_door 0 (Variables|Default|GetLockedMaterial))
    (else
      (Rendering|Material|SetMaterial _sm_door 0 (Variables|Default|GetUnlockedMaterial)))))

(event EventWasToggled
  ;[1 0 0.5482] Door Function Call
  (if (Variables|Default|GetCanBeOpened)
    (Utilities|FlowControl|Sequence
      (:then_0
        ;[1 0 0.5482] Animate Door Opening
        (if (Variables|Default|GetClosedDoor)
          (bind _rotation_angle (Timeline|TL_DoorRotation Play)
            (:Update
              (Transformation|SetRelativeRotation (Variables|Default|GetSM_Door) (Math|Rotator|MakeRotator 0.0 0.0 _rotation_angle) false false)))
          (else
            (Timeline|TL_DoorRotation Reverse))))
      (:then_1
        ;[0 1 0.1445] Play Door Sound
        (Audio|PlaySoundatLocation "/Game/Sounds/door_creak.door_creak" (Transformation|GetWorldLocation (Variables|Default|GetSM_Door)))))))

(fn ConstructionScript)