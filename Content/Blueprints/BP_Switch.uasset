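; Switch actor that gives visual and audio feedback when toggled.
; WasToggled doubles or halves the mesh's Z scale according to IsActive to fake the button indent, then plays a click sound at the mesh.
; It also sets the OnOrOff material parameter to match the state, with BeginPlay always applying the active value.
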(event EventWasToggled
  (bind _sm_switch (Variables|Default|GetSM_Switch))
  (bind _sm_switch_2 (Variables|Default|GetSM_Switch))
  (bind _returnvalue (Transformation|GetWorldScale _sm_switch))
  ;[1 0 0.5482] Change Button Size(Indent)
  (if (Class|Interactable|IsActive)
    (Transformation|SetWorldScale3D _sm_switch (* _returnvalue "1.000000,1.000000,2.000000"))
    (else
      (Transformation|SetWorldScale3D _sm_switch (* _returnvalue "1.000000,1.000000,0.500000"))))
  ;[0 1 0.1445] Play Switch Sound
  (Audio|PlaySoundatLocation "/Game/Sounds/light_click.light_click" (Transformation|GetWorldLocation (Variables|Default|GetSM_Switch)) "0, 0, 0" 0.4)
  ;[1 0.1522 0] Change Material Depending On State
  (if (Class|Interactable|IsActive)
    (Rendering|Material|SetScalarParameterValueonMaterials _sm_switch_2 "OnOrOff" 0.3)
    (else
      (Rendering|Material|SetScalarParameterValueonMaterials _sm_switch_2 "OnOrOff" 0.02))))

(event EventBeginPlay
  ;[1 0.1522 0] Change Material Depending On State
  (Rendering|Material|SetScalarParameterValueonMaterials (Variables|Default|GetSM_Switch) "OnOrOff" 0.3))

(fn ConstructionScript)