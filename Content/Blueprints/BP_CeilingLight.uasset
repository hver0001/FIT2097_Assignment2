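; BP_CeilingLight is a ceiling light Blueprint whose spot light and point light flicker during play.
; On BeginPlay it stores each light's starting intensity, then plays the Flicker timeline.
; Each timeline update multiplies both stored intensities by the Intensity track, so the two lights flicker in sync relative to their own base brightness.
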(event EventBeginPlay
  ;[1 0 0.5482] Get Starting Luminosity
  (Variables|Default|SetStartingIntensity_S (Variables|/Script/Engine.LightComponentBase|GetIntensity (Variables|Default|GetSpotLight)))
  (Variables|Default|SetStartingIntensity_P (Variables|/Script/Engine.LightComponentBase|GetIntensity (Variables|Default|GetPointLight)))
  ;[1 0.1522 0] Flicker Lights
  (bind _intensity (Timeline|Flicker Play)
    (:Update
      (Rendering|Components|Light|SetIntensity (Variables|Default|GetSpotLight) (* (Variables|Default|GetStartingIntensity_S) _intensity))
      (Rendering|Components|Light|SetIntensity (Variables|Default|GetPointLight) (* (Variables|Default|GetStartingIntensity_P) _intensity)))))

(fn ConstructionScript)